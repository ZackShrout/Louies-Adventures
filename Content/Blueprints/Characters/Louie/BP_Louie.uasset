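; Character Blueprint for Louie that performs a timed tongue slurp.
; DoSlurp clears AnimFinished, turns on ShouldSlurp, then spawns a Tongue actor and attaches it to the TongueSpawn component.
; After a SlurpTime delay it destroys the tongue and turns ShouldSlurp off.
; BeginPlay, overlap, Tick and the construction script are empty.
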(event `self.ReceiveBeginPlay`)

(event `self.DoSlurp`
  (set `self.AnimFinished` false)
  (`self.ShouldSlurp` true)
  (bind _returnvalue (`|SpawnActorFromClass` (`self.Tongue`) (`KismetMathLibrary.MakeTransform` (0.0 0.0 0.0)) "Undefined" "MultiplyWithRoot" null null))
  (bind _output_get (set `self.SpawnedTongue` _returnvalue))
  (`self.K2_AttachToComponent` _output_get (`self.TongueSpawn`) "None" "KeepRelative" "KeepRelative" "KeepRelative" false)
  (`KismetSystemLibrary.Delay` (`self.SlurpTime`))
  (`self.K2_DestroyActor` (`self.SpawnedTongue`))
  (`self.ShouldSlurp` false))

(fn `UserConstructionScript`)